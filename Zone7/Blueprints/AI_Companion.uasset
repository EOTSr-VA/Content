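; AI companion pawn that follows the player character, which it caches as BP_ThirdPersonCharacter on BeginPlay.
; While its FollowPlayer flag is set, the FollowPlayer event uses AIMoveTo toward the player at 400 units or more, otherwise targets itself to halt.
; Both moves re-trigger the check after a short delay, forming a polling loop.
; StopMovements reuses the halt branch, so it also feeds back into that loop.
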(event Custom|Follow%20Player
  (if (Variables|Default|GetFollow%20Player%20?)
    (if (>= (Transformation|GetDistanceTo (Variables|Default|GetChar%20Ref)) 4e+02)
      (AI|AIMoveTo self "0, 0, 0" (Variables|Default|GetChar%20Ref) 5.0 false
        (:then
          _))
      (else
        (AI|AIMoveTo self "0, 0, 0" self 5.0 false
          (:then
            _))))
    (Utilities|FlowControl|Delay 0.2)
    (CallFunction|FollowPLAYER)))

(event Custom|Stop%20Movements
  (AI|AIMoveTo self "0, 0, 0" self 5.0 false
    (:then
      (Utilities|FlowControl|Delay 0.2)
      (CallFunction|FollowPLAYER))))

(event EventBeginPlay
  (bind _asbp_third_person_character (Utilities|Casting|CastToBP_ThirdPersonCharacter (Game|GetPlayerCharacter 0)))
  (Variables|Default|SetChar%20Ref _asbp_third_person_character))

(fn ConstructionScript)